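; AI controller for the weak guard (GuardFaible) in the Infiltration game.
; On BeginPlay it runs the guard's behavior tree, then initializes its blackboard.
; It stores the controller actor's own location and rotation, rather than querying the pawn, as the PositionInitial and RotationInitial keys.
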(event EventBeginPlay
  (bind _self self)
  (AI|RunBehaviorTree "/Game/Infiltration/AI/AI_GuardFaible/BT_BehaviourTreeGuardFaible.BT_BehaviourTreeGuardFaible")
  (bind _blackboardcomponent (Class|AIController|UseBlackboard "/Game/Infiltration/AI/AI_GuardFaible/BB_BlackBoardAIGuardFaible.BB_BlackBoardAIGuardFaible"))
  (Variables|Default|SetBlackboard%20Component _blackboardcomponent)
  (AI|Components|Blackboard|SetValueasVector (Variables|Default|GetBlackboard%20Component) (Utilities|Name|MakeLiteralName "PositionInitial") (Transformation|GetActorLocation _self))
  (Class|BlackboardComponent|SetValueasRotator (Variables|Default|GetBlackboard%20Component) (Utilities|Name|MakeLiteralName "RotationInitial") (Transformation|GetActorRotation _self)))

(event EventTick
  (params (DeltaSeconds :type Float%20%28single-precision%29)))

(fn ConstructionScript)